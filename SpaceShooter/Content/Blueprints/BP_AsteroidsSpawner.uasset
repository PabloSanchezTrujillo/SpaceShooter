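; BP_AsteroidsSpawner is an actor that continuously spawns asteroids from a moving spawn point.
; Tick rotates a Pivot component at a configurable rate, while a self-repeating event starts on BeginPlay.
; Each cycle takes an asteroid from a pool, teleport-free moves it to the Spawner component's world location and initializes it.
; The event then calls itself again after a random delay within configurable bounds.
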(event Custom|SpawnAsteroid
  (bind _returnvalue (Class|AsteroidsSpawner|GetAsteroidfromPool))
  (Transformation|SetActorLocation (.AsBP%20Asteroid (Utilities|Casting|CastToBP_Asteroid _returnvalue)) (Transformation|GetWorldLocation (Variables|Default|GetSpawner)) false false)
  (Default|InitAsteroid (.AsBP%20Asteroid (Utilities|Casting|CastToBP_Asteroid _returnvalue)))
  (Utilities|FlowControl|Delay (Math|Random|RandomFloatinRange (Variables|AsteroidsSpawner|GetLapseBetweenAsteroidsMin) (Variables|AsteroidsSpawner|GetLapseBetweenAsteroidsMax)))
  (CallFunction|SpawnAsteroid))

(event EventBeginPlay
  (CallFunction|SpawnAsteroid))

(event EventTick
  (params (DeltaSeconds :type Float%20%28single-precision%29))
  (Transformation|AddLocalRotation (Variables|Default|GetPivot) (* (Variables|AsteroidsSpawner|GetPivotRotation) DeltaSeconds) false false))

(fn ConstructionScript)