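; AsteroidsSpawner is an actor that spawns BP_Asteroid actors endlessly from a rotating point.
; Every tick it rotates its Pivot component by PivotRotation scaled by delta time.
; SpawnAsteroid, started on BeginPlay, spawns an asteroid, moves it to the Spawner component's world location, then calls itself again after a random delay between configurable minimum and maximum lapses.
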(event Custom|SpawnAsteroid
  (bind _spawner (Variables|Default|GetSpawner))
  (bind _returnvalue (Game|SpawnActorfromClass "/Game/Blueprints/BP_Asteroid.BP_Asteroid_C" (Transformation|GetRelativeTransform _spawner) "Undefined" "MultiplyWithRoot" 0 0))
  (Transformation|SetActorLocation _returnvalue (Transformation|GetWorldLocation _spawner) false false)
  (Utilities|FlowControl|Delay (Math|Random|RandomFloatinRange (Variables|Default|GetLapseBetweenAsteroidsMin) (Variables|Default|GetLapseBetweenAsteroidsMax)))
  (CallFunction|SpawnAsteroid))

(event EventBeginPlay
  (CallFunction|SpawnAsteroid))

(event EventTick
  (params (DeltaSeconds :type Float%20%28single-precision%29))
  (Transformation|AddLocalRotation (Variables|Default|GetPivot) (* (Variables|Default|GetPivotRotation) DeltaSeconds) false false))

(fn ConstructionScript)