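; Player spaceship Blueprint that moves by pitching its MovementPivot, with a temporary speed boost.
; BeginPlay adds the IMC_Spaceship Enhanced Input context; left, right and dead-zoned stick actions add local rotation scaled by RotationSpeed, without delta time.
; Boost raises RotationSpeed for a set duration while a parallel delay gates its cooldown.
; Joystick reading, HUD creation and debug print nodes are left unconnected.
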(event Input|EnhancedActionEvents|EnhancedInputActionIA_SpaceshipBoost
  (params (ActionValue :type Boolean) (ElapsedSeconds :type Float%20%28double-precision%29) (TriggeredSeconds :type Float%20%28double-precision%29) (InputAction :type Input%20Action%20Object%20Reference :default "/Game/Inputs/SpaceshipActions/IA_SpaceshipBoost.IA_SpaceshipBoost"))
  ;[1 1 1 1 40] Spaceship boost
  (:Started
    (if (Variables|Default|GetBoostAvaliable)
      (Utilities|FlowControl|Sequence
        (:then_0
          (Variables|Default|SetBoostAvaliable false)
          (Variables|Default|SetRotationSpeed (+ (Variables|Default|GetRotationSpeed) (Variables|Default|GetBoostSpeed)))
          (Utilities|FlowControl|Delay (Variables|Default|GetBoostDuration))
          (Variables|Default|SetRotationSpeed (- (Variables|Default|GetRotationSpeed) (Variables|Default|GetBoostSpeed))))
        (:then_1
          (Utilities|FlowControl|Delay (Variables|Default|GetBoostCooldown))
          (Variables|Default|SetBoostAvaliable true))))))

(event Input|EnhancedActionEvents|EnhancedInputActionIA_SpaceshipLeftMovement
  (params (ActionValue :type Boolean) (ElapsedSeconds :type Float%20%28double-precision%29) (TriggeredSeconds :type Float%20%28double-precision%29) (InputAction :type Input%20Action%20Object%20Reference :default "/Game/Inputs/SpaceshipActions/IA_SpaceshipLeftMovement.IA_SpaceshipLeftMovement"))
  ;[1 1 1 1 40] Spaceship movement
  (Transformation|AddLocalRotation (Variables|Default|GetMovementPivot) (Math|Rotator|MakeRotator 0.0 (* (Variables|Default|GetRotationSpeed) -1.0) 0.0) false false))

(event Input|EnhancedActionEvents|EnhancedInputActionIA_SpaceshipRightMovement
  (params (ActionValue :type Boolean) (ElapsedSeconds :type Float%20%28double-precision%29) (TriggeredSeconds :type Float%20%28double-precision%29) (InputAction :type Input%20Action%20Object%20Reference :default "/Game/Inputs/SpaceshipActions/IA_SpaceshipRightMovement.IA_SpaceshipRightMovement"))
  ;[1 1 1 1 40] Spaceship movement
  (Transformation|AddLocalRotation (Variables|Default|GetMovementPivot) (Math|Rotator|MakeRotator 0.0 (Variables|Default|GetRotationSpeed) 0.0) false false))

(event Input|EnhancedActionEvents|EnhancedInputActionIA_SpaceshipStickMovement
  (params (ActionValue :type Float%20%28double-precision%29) (ElapsedSeconds :type Float%20%28double-precision%29) (TriggeredSeconds :type Float%20%28double-precision%29) (InputAction :type Input%20Action%20Object%20Reference :default "/Game/Inputs/SpaceshipActions/IA_SpaceshipStickMovement.IA_SpaceshipStickMovement"))
  (bind _stickblindangle (Variables|Default|GetStickBlindAngle))
  ;[1 1 1 1 40] Spaceship movement
  (if (or (< ActionValue (* _stickblindangle -1.0)) (> ActionValue _stickblindangle))
    (Transformation|AddLocalRotation (Variables|Default|GetMovementPivot) (Math|Rotator|MakeRotator 0.0 (* ActionValue (Variables|Default|GetRotationSpeed)) 0.0) false false)))

(event EventBeginPlay
  (bind _returnvalue (Game|GetPlayerController 0))
  (bind _returnvalue_2 (PlayerController|LocalPlayerSubsystems|GetEnhancedInputLocalPlayerSubsystem _returnvalue))
  (Utilities|IsValid _returnvalue_2
    (:Is%20Valid
      (Input|AddMappingContext _returnvalue_2 "/Game/Inputs/SpaceshipActions/IMC_Spaceship.IMC_Spaceship" 0 "(bIgnoreAllPressedKeysUntilRelease=True,bForceImmediately=False,bNotifyUserSettings=False)"))))

(event Collision|EventActorBeginOverlap
  (params (OtherActor :type Actor%20Object%20Reference)))

(event EventTick
  (params (DeltaSeconds :type Float%20%28single-precision%29)))

(fn ConstructionScript)