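; BP_Asteroid is an asteroid actor that tumbles as it drifts along the Y axis and reacts to hitting the player.
; The construction script randomizes spin and speed, putting faster roll in the higher speed band.
; Tick applies both values scaled by delta time, moving the root without sweep.
; Collision overlaps go through CollisionWithPlayer, and a true result plays a 2D explosion sound.
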(event OnComponentBeginOverlap(Collision)
  (params (OverlappedComponent :type Primitive%20Component%20Object%20Reference) (OtherActor :type Actor%20Object%20Reference) (OtherComp :type Primitive%20Component%20Object%20Reference) (OtherBodyIndex :type Integer) (bFromSweep :type Boolean) (SweepResult :type Hit%20Result%20Structure%20%28by%20ref%29))
  (bind _returnvalue (Class|Asteroid|CollisionwithPlayer OtherActor))
  (if _returnvalue
    (Audio|PlaySound2D "/Game/Sounds/Explosion.Explosion" 1.0 1.0 0.0 0 0)))

(event EventTick
  (params (DeltaSeconds :type Float%20%28single-precision%29))
  (Transformation|AddLocalRotation (Variables|Default|GetSM_Asteroid) (* (Variables|Default|GetAsteroidRotation) DeltaSeconds) false false)
  (Transformation|AddRelativeLocation (Variables|Default|GetDefaultSceneRoot) (* (Variables|Default|GetAsteroidMovement) DeltaSeconds) false false))

(fn ConstructionScript
  (bind _output_get (Variables|Default|SetAsteroidRotation (Math|Rotator|MakeRotator (Math|Random|RandomFloatinRange 3e+02 4e+02) (Math|Random|RandomFloatinRange 1.5e+02 3e+02) (Math|Random|RandomFloatinRange 5e+01 2e+02))))
  (if (< (.Roll (Math|Rotator|BreakRotator _output_get)) 3.5e+02)
    (Variables|Default|SetAsteroidMovement (Math|Vector|MakeVector 0.0 (Math|Random|RandomFloatinRange 3e+02 4e+02) 0.0))
    (else
      (Variables|Default|SetAsteroidMovement (Math|Vector|MakeVector 0.0 (Math|Random|RandomFloatinRange 4e+02 5e+02) 0.0)))))